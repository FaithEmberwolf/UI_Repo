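; AC_ItemData is an item component that lets its owning actor be picked up into a player's inventory.
; On BeginPlay it turns on replication for the owner.
; Interactwith passes the item's row name and quantity to the player's ACInventorySystem and destroys the owner if the add succeeds.
; LookAt returns an empty string.
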(event `self.ReceiveBeginPlay`
  (`Actor.SetReplicates` (`self.GetOwner`) true))

(event `/Game/InventorySystem/I_InteractionInterface.InteractWith`
  (params (PlayerCharacter :type "/Game/ThirdPerson/Blueprints/BP_ThirdPersonCharacter Object Reference"))
  (bind _ac_inventorysystem (`/Game/ThirdPerson/Blueprints/BP_ThirdPersonCharacter.AC_InventorySystem` PlayerCharacter))
  (bind (_factid_datatable _factid_rowname) (break `DataTableRowHandle` (`self.FactID`)))
  (`/Engine/EditorBlueprintResources/StandardMacros.IsValid` _ac_inventorysystem
    (:`Is Valid`
      (bind _success (`/Game/InventorySystem/AC_InventorySystem.AddToInventory` _ac_inventorysystem _factid_rowname (`self.Quantity`)))
      (if _success
        (`Actor.K2_DestroyActor` (`self.GetOwner`))))))

(fn `LookAt`
  (returns (Message :type Text))
  (return ""))