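; Inventory component that stores fact items in fixed-size slots and handles the owning character's interaction with world items.
; Each tick, a forward sphere trace tracks the looked-at actor, and the interact input passes it through a server event to its AC_ItemData.
; Adding fills stacks up to DT_FactData limits, then empty slots, though AddToStack reads Content by Quantity instead of Index.
; Removal is an empty stub, and key 1 prints contents for debugging.
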(event `self.ReceiveBeginPlay`
  (`KismetArrayLibrary.Array_Resize` (`self.Content`) (`self.InventorySize`)))

(event `self.ReceiveTick`
  (params (DeltaSeconds :type "Float (single-precision)"))
  (`self.InteractionTrace`))

(event `EnhancedInput|/Game/ThirdPerson/Input/Actions/IA_Interact`
  (params (ActionValue :type "Vector2D Structure") (ElapsedSeconds :type "Float (double-precision)") (TriggeredSeconds :type "Float (double-precision)") (InputAction :type "InputAction Object Reference" :default "/Game/ThirdPerson/Input/Actions/IA_Interact.IA_Interact"))
  (:`Started`
    (bind _lookat (`self.LookAt`)
      (:`then`
        (`self.Server_Intereact` _lookat))
      (:`else`))))

(event `Server_Intereact`
  (params (Target :type "Actor Object Reference"))
  (bind _returnvalue (`Actor.GetComponentByClass` Target "/Game/InventorySystem/AC_ItemData.AC_ItemData_C"))
  (`/Engine/EditorBlueprintResources/StandardMacros.IsValid` _returnvalue
    (:`Is Valid`
      (message `/Game/InventorySystem/I_InteractionInterface.InteractWith` _returnvalue (cast `/Game/ThirdPerson/Blueprints/BP_ThirdPersonCharacter` (`self.GetOwner`) :!pure true)))))

(event `Key|One`
  (params (Key :type "Key Structure"))
  (:`Pressed`
    (`self.DEBUG_PrintContent`)))

(fn `AddToInventory`
  (params (FactID :type Name) (Quantity :type Integer))
  (returns (Success :type Boolean) (`Quantity Remaining` :type Integer))
  (locals (Local_QuantityRemaining :type Integer) (Local_HasFailed :type Boolean))
  (set `local.Local_QuantityRemaining` Quantity)
  (while (and (> (`local.Local_QuantityRemaining`) 0) (not (`local.Local_HasFailed`)))
    (bind (_index _foundslot) (`self.FindSlot` (`local.FactID`)))
    (if _foundslot
      (`self.AddToStack` _index 1)
      (`/Engine/EditorBlueprintResources/StandardMacros.DecrementInt` (`local.Local_QuantityRemaining`))
      (elif (`self.AnyEmptySlotsAvalible`)
        (`self.CreateNewStack` (`local.FactID`) 1)
        (if true
          (`/Engine/EditorBlueprintResources/StandardMacros.DecrementInt` (`local.Local_QuantityRemaining`))
          (else
            (set `local.Local_HasFailed` true)))
        (else
          (set `local.Local_HasFailed` true)))))
  (return (not (`local.Local_HasFailed`)) (`local.Local_QuantityRemaining`)))

(fn `AddToStack`
  (params (Index :type Integer) (Quantity :type Integer))
  (bind (_output_factid _output_itemquantity) (break `/Game/InventorySystem/F_DisplayStruct` (`|GetArrayItem` (`self.Content`) Quantity)))
  (`KismetArrayLibrary.Array_Set` (`self.Content`) Index (make `/Game/InventorySystem/F_DisplayStruct` _output_factid (+ _output_itemquantity (`local.Quantity`)))))

(fn `AnyEmptySlotsAvalible`
  (returns (HasEmptySlot :type Boolean) (EmptyIndex :type Integer))
  (for (_array_element _array_index) (`self.Content`)
    (if (== (`.ItemQuantity_7_258029D948A65F838DBF3682F96908F4` (break `/Game/InventorySystem/F_DisplayStruct` _array_element)) 0)
      (return true _array_index)))
  (return false -1))

(fn `CreateNewStack`
  (params (FactID :type Name) (Quantity :type Integer))
  (returns (Success :type Boolean))
  (bind (_hasemptyslot _emptyindex) (`self.AnyEmptySlotsAvalible`))
  (if _hasemptyslot
    (`KismetArrayLibrary.Array_Set` (`self.Content`) _emptyindex (make `/Game/InventorySystem/F_DisplayStruct` (`local.FactID`) (`local.Quantity`)))
    (return true)
    (else
      (return false))))

(fn `DEBUG_PrintContent`
  (for (_array_element _array_index) (`self.Content`)
    (bind (_factid _itemquantity) (break `/Game/InventorySystem/F_DisplayStruct` _array_element))
    (`KismetSystemLibrary.PrintString` (`KismetStringLibrary.Concat_StrStr` (`KismetStringLibrary.Conv_IntToString` _array_index) " : " (`KismetStringLibrary.Conv_NameToString` _factid) " & " (`KismetStringLibrary.Conv_IntToString` _itemquantity)))))

(fn `FindSlot`
  (params (FactID :type Name))
  (returns (Index :type Integer) (FoundSlot :type Boolean))
  (bind _factid (`local.FactID`))
  (for (_array_element _array_index) (`self.Content`)
    (bind (_factid_2 _itemquantity) (break `/Game/InventorySystem/F_DisplayStruct` _array_element))
    (if (== _factid_2 _factid)
      (if (< _itemquantity (`self.GetMaxStackSize` _factid))
        (return _array_index true))))
  (return -1 false))

(fn `GetMaxStackSize`
  (params (FactID :type Name))
  (returns (StackSize :type Integer))
  (bind _returnvalue (`|GetDataTableRow` "/Game/InventorySystem/DT_FactData.DT_FactData" FactID)
    (:`then`
      (return (`.StackSize_17_5AC98A6247180087AF1847AA220CC947` (break `/Game/InventorySystem/F_FactStruct` _returnvalue))))
    (:`RowNotFound`
      (return -1))))

(fn `InteractionTrace`
  (bind _returnvalue (`GameplayStatics.GetPlayerCharacter` 0))
  (bind _returnvalue_2 (`Actor.K2_GetActorLocation` _returnvalue))
  (bind (_outhit _returnvalue_3) (`KismetSystemLibrary.SphereTraceSingle` _returnvalue_2 (+ _returnvalue_2 (* (`Actor.GetActorForwardVector` _returnvalue) (`self.InteractionRange`))) 15.0 "TraceTypeQuery3" false (`|MakeArray` (`self.GetOwner`))))
  (if _returnvalue_3
    (bind (_bblockinghit _binitialoverlap _time _distance _location _impactpoint _normal _impactnormal _physmat _hitactor) (`GameplayStatics.BreakHitResult` _outhit))
    (if (!= _hitactor (`self.LookAt`))
      (bind _output_get (set `self.LookAt` _hitactor))
      (bind _message (message `/Game/InventorySystem/I_InteractionInterface.LookAt` _output_get))
      (`KismetSystemLibrary.PrintString` (`KismetTextLibrary.Conv_TextToString` _message)))
    (else
      (set `self.LookAt` null))))

(fn `RemoveFromInventory`)